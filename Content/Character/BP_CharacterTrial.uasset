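; Trial side-scrolling player character that moves along world X, flips to face its acceleration direction, and switches between walk and run speeds.
; Tick drives one-way platforms: a downward trace while falling toggles capsule collision on the Vehicle channel, and an input forces overlap to drop through.
; Coyote time uses a retriggerable delay on walking off ledges, feeding an overridden CanJumpInternal.
; The change-mode input only looks up the follow camera, without acting on it.
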(event Input|EnhancedActionEvents|EnhancedInputActionIA_Move
  (params (ActionValue :type Float%20%28double-precision%29) (ElapsedSeconds :type Float%20%28double-precision%29) (TriggeredSeconds :type Float%20%28double-precision%29) (InputAction :type Input%20Action%20Object%20Reference :default "/Game/Inputs/IA_Move.IA_Move"))
  (bind _returnvalue (Pawn|GetController))
  (Pawn|Input|AddMovementInput "1.000000,0.000000,0.000000" ActionValue false)
  (Math|Float|CompareFloat (.x (Pawn|Components|CharacterMovement|GetCurrentAcceleration (Variables|Character|GetCharacterMovement))) 0.0
    (:>
      (Pawn|SetControlRotation _returnvalue (Math|Rotator|MakeRotator 0.0 0.0 0.0)))
    (:<
      (Pawn|SetControlRotation _returnvalue (Math|Rotator|MakeRotator 0.0 0.0 1.8e+02)))))

(event Input|EnhancedActionEvents|EnhancedInputActionIA_Jump
  (params (ActionValue :type Boolean) (ElapsedSeconds :type Float%20%28double-precision%29) (TriggeredSeconds :type Float%20%28double-precision%29) (InputAction :type Input%20Action%20Object%20Reference :default "/Game/Inputs/IA_Jump.IA_Jump"))
  (:Started
    (Character|Jump)))

(event Input|EnhancedActionEvents|EnhancedInputActionIA_DesablePlatform
  (params (ActionValue :type Float%20%28double-precision%29) (ElapsedSeconds :type Float%20%28double-precision%29) (TriggeredSeconds :type Float%20%28double-precision%29) (InputAction :type Input%20Action%20Object%20Reference :default "/Game/Inputs/IA_DesablePlatform.IA_DesablePlatform"))
  (:Started
    (Variables|Default|SetDisableCollision true :!label _label)
    (Collision|SetCollisionResponsetoChannel (Variables|Default|GetCapsuleComponent) "ECC_Vehicle" "ECR_Overlap")
    (Utilities|FlowControl|Delay 0.0)
    (Variables|Default|SetDisableCollision false))
  (:Ongoing
    (goto _label)))

(event Input|EnhancedActionEvents|EnhancedInputActionIA_Run
  (params (ActionValue :type Boolean) (ElapsedSeconds :type Float%20%28double-precision%29) (TriggeredSeconds :type Float%20%28double-precision%29) (InputAction :type Input%20Action%20Object%20Reference :default "/Game/Inputs/IA_Run.IA_Run"))
  (bind _charactermovement (Variables|Character|GetCharacterMovement))
  (:Triggered
    (Variables|/Script/Engine.CharacterMovementComponent|SetMaxWalkSpeed _charactermovement (Variables|Default|GetSpeedRun)))
  (:Completed
    (Variables|/Script/Engine.CharacterMovementComponent|SetMaxWalkSpeed _charactermovement (Variables|Default|GetSpeedWalk))))

(event Input|EnhancedActionEvents|EnhancedInputActionIA_ChangeMode
  (params (ActionValue :type Boolean) (ElapsedSeconds :type Float%20%28double-precision%29) (TriggeredSeconds :type Float%20%28double-precision%29) (InputAction :type Input%20Action%20Object%20Reference :default "/Game/Inputs/IA_ChangeMode.IA_ChangeMode"))
  (:Started
    (bind _returnvalue (Actor|GetActorOfClass "/Game/Camera/BP_CameraFollowsPlayer.BP_CameraFollowsPlayer_C"))
    (Utilities|IsValid _returnvalue)))

(event EventBeginPlay
  (CallFunction|AddMappingContext))

(event EventGetCameraFilm
  (params (CameraFilm :type Integer))
  (Variables|Default|SetCameraFilm (+ CameraFilm (Variables|Default|GetCameraFilm))))

(event EventOnWalkingOffLedge
  (params (PreviousFloorImpactNormal :type Vector%20%28by%20ref%29 :default "0, 0, 0") (PreviousFloorContactNormal :type Vector%20%28by%20ref%29 :default "0, 0, 0") (PreviousLocation :type Vector%20%28by%20ref%29 :default "0, 0, 0") (TimeDelta :type Float%20%28single-precision%29))
  (Variables|CoyoteTime|SetIsInCoyoteTime? true)
  (Utilities|FlowControl|RetriggerableDelay (Variables|CoyoteTime|GetCoyoteTime))
  (Variables|CoyoteTime|SetIsInCoyoteTime? false))

(event EventTick
  (params (DeltaSeconds :type Float%20%28single-precision%29))
  (CallFunction|CheckPlatforms)
  (CallFunction|UpdateSpeed))

(fn ConstructionScript)

(fn AddMappingContext
  (bind _asplayer_controller (Utilities|Casting|CastToPlayerController (Pawn|GetController)))
  (Input|AddMappingContext (PlayerController|LocalPlayerSubsystems|GetEnhancedInputLocalPlayerSubsystem _asplayer_controller) "/Game/MappingContext/IMC_Lvl1CameraLife.IMC_Lvl1CameraLife" 0 "(bIgnoreAllPressedKeysUntilRelease=True,bForceImmediately=False,bNotifyUserSettings=False)"))

(fn CheckPlatforms
  (if (AI|Components|NavMovement|IsFalling (Variables|Character|GetCharacterMovement))
    (bind _returnvalue (Collision|LineTraceForObjects (+ (Transformation|GetActorLocation) "0.000000,0.000000,-70.000000") (- (Transformation|GetActorLocation) (* (Math|Vector|VectorDown) (* (Variables|Default|GetDetectDistance) -1.0))) (Utilities|Array|MakeArray "ObjectTypeQuery5") false 0 "None"))
    (if (Math|Boolean|ANDBoolean _returnvalue (< (.z (Transformation|GetVelocity)) 0.0) (not (Variables|Default|GetDisableCollision)))
      (Collision|SetCollisionResponsetoChannel (Variables|Default|GetCapsuleComponent) "ECC_Vehicle" "ECR_Block")
      (else
        (Collision|SetCollisionResponsetoChannel (Variables|Default|GetCapsuleComponent) "ECC_Vehicle" "ECR_Overlap")))))

(fn UpdateSpeed
  (Variables|/Script/Engine.CharacterMovementComponent|SetMaxWalkSpeed (Variables|Character|GetCharacterMovement) (Math|Float|SelectFloat (Variables|Default|GetSpeedRun) (Variables|Default|GetSpeedWalk) (Input|EnhancedActionValues|GetIA_Run))))

(fn CanJumpInternal
  (bind _returnvalue (|CallParentFunction))
  (return (or _returnvalue (Variables|CoyoteTime|GetIsInCoyoteTime?))))