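; Side-view camera actor that follows the BP_CharacterTrial player across the X and Z axes within set limits.
; On BeginPlay it finds the player, then each Tick interpolates toward the player's clamped position at CameraSpeed, keeping its own Y fixed.
; It also holds functions that toggle between fullscreen at desktop resolution and windowed mode at a given resolution via GameUserSettings, though none are called within this file.
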(event EventBeginPlay
  (bind _returnvalue (Actor|GetActorOfClass "/Game/Character/BP_CharacterTrial.BP_CharacterTrial_C"))
  (Variables|Default|SetPlayer _returnvalue))

(event EventTick
  (params (DeltaSeconds :type Float%20%28single-precision%29))
  (bind _returnvalue (Transformation|GetActorLocation))
  (bind _player (Variables|Default|GetPlayer))
  (bind _returnvalue_2 (Transformation|GetActorLocation _player))
  (Transformation|SetActorLocation (Math|Interpolation|VInterpTo (Math|Vector|MakeVector (.x _returnvalue) (.y _returnvalue) (.z _returnvalue)) (Math|Vector|MakeVector (Math|Float|Clamp(Float) (.x _returnvalue_2) (Variables|Limits|GetLeftLimit) (Variables|Limits|GetRightLimit)) (.y _returnvalue) (Math|Float|Clamp(Float) (.z _returnvalue_2) (Variables|Limits|GetInferiorLimit%20) (Variables|Limits|GetSuperiorLimit))) DeltaSeconds (Variables|Default|GetCameraSpeed)) false false))

(fn ConstructionScript)

(fn ChangetoWindowMode
  (params (Resolution :type Int%20Point%20Structure))
  (bind _returnvalue (Settings|GetGameUserSettings))
  (Class|GameUserSettings|SetFullscreenMode _returnvalue "Windowed")
  (Class|GameUserSettings|SetScreenResolution _returnvalue Resolution)
  (Class|GameUserSettings|ApplySettings _returnvalue false))

(fn ChangetoFullscreen
  (bind _returnvalue (Settings|GetGameUserSettings))
  (Class|GameUserSettings|SetFullscreenMode _returnvalue "Fullscreen")
  (Class|GameUserSettings|SetScreenResolution _returnvalue (Class|GameUserSettings|GetDesktopResolution _returnvalue))
  (Class|GameUserSettings|ApplySettings _returnvalue false))

(fn ChangeScreenMode
  (params (Resolution :type Int%20Point%20Structure))
  (bind _returnvalue (Settings|GetGameUserSettings))
  (switch Utilities|FlowControl|Switch|SwitchonEWindowMode (Class|GameUserSettings|GetFullscreenMode _returnvalue)
    (:Fullscreen
      (CallFunction|ChangetoWindowMode Resolution :!label _label))
    (:WindowedFullscreen
      (goto _label))
    (:Windowed
      (CallFunction|ChangetoFullscreen))))